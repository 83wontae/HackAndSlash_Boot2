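; BP_HSGameMode is the hack-and-slash game mode that drives the opening phase transition of a match.
; On BeginPlay it sets the BP_HSGameState to Ready.
; Each Tick it switches on the current state, and during Ready it moves to Play once the game state's TotalDeltaSeconds reaches a five-second threshold.
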(event `self.ReceiveBeginPlay`
  (bind _asbp_hsgame_state (cast `/Game/HackAndSlash/GameMode/BP_HSGameState` (`GameplayStatics.GetGameState`)))
  (`/Game/HackAndSlash/GameMode/BP_HSGameState.ChangeGameState` _asbp_hsgame_state "NewEnumerator1"))

(event `self.ReceiveTick`
  (params (DeltaSeconds :type "Float (single-precision)"))
  (bind _asbp_hsgame_state (cast `/Game/HackAndSlash/GameMode/BP_HSGameState` (`GameplayStatics.GetGameState`)))
  (switch `/Game/HackAndSlash/GameMode/EN_GameState` (`/Game/HackAndSlash/GameMode/BP_HSGameState.GameState` _asbp_hsgame_state)
    (:`NewEnumerator1`
      (`self.UpdateReady` _asbp_hsgame_state))))

(fn `UpdateReady`
  (params (GameState :type "/Game/HackAndSlash/GameMode/BP_HSGameState Object Reference"))
  (if (>= (`/Game/HackAndSlash/GameMode/BP_HSGameState.TotalDeltaSeconds` GameState) 5.0)
    (`/Game/HackAndSlash/GameMode/BP_HSGameState.ChangeGameState` GameState "NewEnumerator2")))

(fn `UserConstructionScript`)