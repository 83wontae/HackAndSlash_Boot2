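; A hack-and-slash skill actor that circles its instigator and repeatedly damages monsters it touches.
; Each Tick it snaps to the instigator's location and rotates its spring arm by a fixed step, not scaled by delta time.
; A looping timer started on BeginPlay applies damage to every BP_MonsterBase overlapping its sphere, crediting the instigator and its controller.
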(event `self.ReceiveTick`
  (params (DeltaSeconds :type "Float (single-precision)"))
  (`self.MoveAround`))

(event `self.ReceiveBeginPlay`
  (`parent.ReceiveBeginPlay`)
  (`KismetSystemLibrary.K2_SetTimer` null "DoApplyDamage" 0.1 true))

(fn `DoApplyDamage`
  (bind _instigator (`self.Instigator`))
  (for _array_element (`PrimitiveComponent.GetOverlappingActors` (`self.Sphere`) "/Game/HackAndSlash/Monsters/BP_MonsterBase.BP_MonsterBase_C")
    (`GameplayStatics.ApplyDamage` _array_element 10.0 (`Pawn.GetController` _instigator) _instigator)))

(fn `MoveAround`
  (`SceneComponent.K2_AddRelativeRotation` (`self.SpringArm`) (struct :`Yaw` 2.0) false false)
  (`self.K2_SetActorLocation` (`self.K2_GetActorLocation` (`self.Instigator`))))

(fn `UserConstructionScript`
  (`parent.UserConstructionScript`))