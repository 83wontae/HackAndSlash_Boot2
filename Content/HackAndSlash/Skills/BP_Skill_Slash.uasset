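; BP_Skill_Slash is a hack-and-slash skill actor that deals area damage to monsters when it spawns.
; On BeginPlay it attaches itself to its Instigator character and sets its relative transform.
; It then makes a single overlap check with its Sphere, applying fixed damage to each BP_MonsterBase found and crediting the Instigator and its controller.
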(event `self.ReceiveBeginPlay`
  (`parent.ReceiveBeginPlay`)
  (`self.AttachToChar`)
  (`self.DoApplyDamage`))

(fn `AttachToChar`
  (bind _ascharacter (cast `Character` (`self.Instigator`)))
  (`self.K2_AttachToActor` _ascharacter "None" "KeepRelative" "KeepRelative" "KeepRelative")
  (`self.K2_SetActorRelativeTransform` (`KismetMathLibrary.MakeTransform` (0.0 0.0 0.0))))

(fn `DoApplyDamage`
  (bind _instigator (`self.Instigator`))
  (for _array_element (`PrimitiveComponent.GetOverlappingActors` (`self.Sphere`) "/Game/HackAndSlash/Monsters/BP_MonsterBase.BP_MonsterBase_C")
    (`GameplayStatics.ApplyDamage` _array_element 10.0 (`Pawn.GetController` _instigator) _instigator)))

(fn `UserConstructionScript`
  (`parent.UserConstructionScript`))