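; Homing projectile skill for the hack-and-slash game that seeks a nearby target and explodes on overlap.
; Each tick it sphere-traces around its Arrow for a target, smoothly turns toward it using X/Y positions only, and moves forward without sweeping.
; Mesh overlap applies radial damage that ignores the Instigator, spawns an explosion effect and destroys the actor.
; The search trace and damage radius are drawn as debug shapes.
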(event `self.ReceiveTick`
  (params (DeltaSeconds :type "Float (single-precision)"))
  (if (not (`self.IsActorBeingDestroyed`))
    (`self.FindTarget`)
    (`self.RotateToTarget` DeltaSeconds)
    (`self.MoveForward` DeltaSeconds)))

(event `self.StaticMesh.OnComponentBeginOverlap`
  (params (OverlappedComponent :type "PrimitiveComponent Object Reference") (OtherActor :type "Actor Object Reference") (OtherComp :type "PrimitiveComponent Object Reference") (OtherBodyIndex :type Integer) (bFromSweep :type Boolean) (SweepResult :type "HitResult Structure (by ref)"))
  (bind (_returnvalue_location _returnvalue_rotation) (`KismetMathLibrary.BreakTransform` (`SceneComponent.K2_GetComponentToWorld` (`self.Arrow`))))
  (`self.DoApplyDamage`)
  (`GameplayStatics.SpawnEmitterAtLocation` "/Game/StarterContent/Particles/P_Explosion.P_Explosion" _returnvalue_location _returnvalue_rotation (2.0 2.0 2.0))
  (`self.K2_DestroyActor`))

(fn `DoApplyDamage`
  (bind _instigator (`self.Instigator`))
  (`KismetSystemLibrary.DrawDebugSphere` (`SceneComponent.K2_GetComponentLocation` (`self.Arrow`)) (`self.Radius`) 12 (struct :`R` 1.0 :`A` 1.0) 3.0 1.0)
  (`GameplayStatics.ApplyRadialDamage` 50.0 (`SceneComponent.K2_GetComponentLocation` (`self.Arrow`)) (`self.Radius`) null (`|MakeArray` _instigator :!type "Actor Object Reference") self (`Pawn.GetController` _instigator)))

(fn `FindTarget`
  (bind _returnvalue (`SceneComponent.K2_GetComponentLocation` (`self.Arrow`)))
  (bind (_outhit _returnvalue_2) (`KismetSystemLibrary.SphereTraceSingleForObjects` :`Start` _returnvalue :`End` _returnvalue :`Radius` 1000.0 :`ObjectTypes` (`|MakeArray` "ObjectTypeQuery7" :!type "EObjectTypeQuery Enum") :`DrawDebugType` "ForOneFrame"))
  (if _returnvalue_2
    (set `self.Target` (`.HitActor` (`GameplayStatics.BreakHitResult` _outhit)))))

(fn `MoveForward`
  (params (DeltaSeconds :type "Float (single-precision)"))
  (bind _arrow (`self.Arrow`))
  (`SceneComponent.K2_AddWorldOffset` _arrow (* (`SceneComponent.GetForwardVector` _arrow) (* DeltaSeconds (`self.Speed`))) false false))

(fn `RotateToTarget`
  (params (DeltaSeconds :type "Float (double-precision)"))
  (bind _target (`self.Target`)
    (:`then`
      (bind _arrow (`self.Arrow`)
        (:`then`
          (if (not (`ActorComponent.IsBeingDestroyed` _arrow))
            (bind (_returnvalue_x _returnvalue_y) (`KismetMathLibrary.BreakVector` (`SceneComponent.K2_GetComponentLocation` _arrow)))
            (bind (_returnvalue_x_2 _returnvalue_y_2) (`KismetMathLibrary.BreakVector` (`self.K2_GetActorLocation` _target)))
            (`SceneComponent.K2_SetWorldRotation` (`self.Arrow`) (`KismetMathLibrary.RInterpTo` (`SceneComponent.K2_GetComponentRotation` _arrow) (`KismetMathLibrary.FindLookAtRotation` (`KismetMathLibrary.MakeVector` _returnvalue_x _returnvalue_y) (`KismetMathLibrary.MakeVector` _returnvalue_x_2 _returnvalue_y_2)) (`local.DeltaSeconds`) 10.0) false false)))
        (:`else`)))
    (:`else`)))

(fn `UserConstructionScript`
  (`parent.UserConstructionScript`))